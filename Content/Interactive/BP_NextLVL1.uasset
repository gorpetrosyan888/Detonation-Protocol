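; BP_NextLVL1 is an interactive sliding double door that opens when its OpenDoors event is called, playing a 2D sci-fi door sound.
; EnumRef selects the slide axis, X or Y, with a separate pair of timelines for each.
; The first timeline restarts and moves SMDoor01 along that axis, and its Update also calls Play on the second, which moves SMDoor02 while preserving the other coordinates.
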(event EventOpenDoors
  (bind _sm_door_02 (Variables|Default|GetSM_Door_02))
  (bind _sm_door_01 (Variables|Default|GetSM_Door_01))
  (bind _sm_door_01_2 (Variables|Default|GetSM_Door_01))
  (bind _sm_door_02_2 (Variables|Default|GetSM_Door_02))
  (bind _relativelocation (Variables|/Script/Engine.SceneComponent|GetRelativeLocation _sm_door_02_2))
  (bind _relativelocation_2 (Variables|/Script/Engine.SceneComponent|GetRelativeLocation _sm_door_01_2))
  (bind _relativelocation_3 (Variables|/Script/Engine.SceneComponent|GetRelativeLocation _sm_door_01))
  (bind _relativelocation_4 (Variables|/Script/Engine.SceneComponent|GetRelativeLocation _sm_door_02))
  (switch Utilities|FlowControl|Switch|SwitchonE_DoorChoose (Variables|Default|GetEnumRef)
    (:NewEnumerator0
      (Audio|PlaySound2D "/Game/SFX/543404__alexo400__sci_fi_door.543404__alexo400__sci_fi_door" 1.0 1.0 0.0 0 0)
      (bind _newtrack_0 (Timeline|Timeline_0 PlayFromStart)
        (:Update
          (Transformation|SetRelativeLocation (Variables|Default|GetSM_Door_01) (Math|Vector|MakeVector _newtrack_0 (.y _relativelocation_3) (.z _relativelocation_3)) false false)
          (bind _newtrack_0_2 (Timeline|Timeline Play)
            (:Update
              (Transformation|SetRelativeLocation (Variables|Default|GetSM_Door_02) (Math|Vector|MakeVector _newtrack_0_2 (.y _relativelocation_4) (.z _relativelocation_4)) false false))))))
    (:NewEnumerator1
      (Audio|PlaySound2D "/Game/SFX/543404__alexo400__sci_fi_door.543404__alexo400__sci_fi_door" 1.0 1.0 0.0 0 0)
      (bind _newtrack_0_3 (Timeline|Timeline_2 PlayFromStart)
        (:Update
          (Transformation|SetRelativeLocation (Variables|Default|GetSM_Door_01) (Math|Vector|MakeVector (.x _relativelocation_2) _newtrack_0_3 (.z _relativelocation_2)) false false)
          (bind _newtrack_0_4 (Timeline|Timeline_1 Play)
            (:Update
              (Transformation|SetRelativeLocation (Variables|Default|GetSM_Door_02) (Math|Vector|MakeVector (.x _relativelocation) _newtrack_0_4 (.z _relativelocation)) false false))))))))

(fn ConstructionScript)