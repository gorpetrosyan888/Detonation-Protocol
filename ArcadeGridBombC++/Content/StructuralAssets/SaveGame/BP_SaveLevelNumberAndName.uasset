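; SaveGame Blueprint that persists the level number and level name.
; Each save function stores its value on the object and writes the whole object to that value's own slot, LevelNumberSlot or LevelNameSlot.
; Each load function checks that its slot exists, casts the loaded object to this class, then copies only its field back into this instance and returns it.
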(fn SaveLevelNumber
  (params (NewParam :type Integer))
  (bind _output_get (Variables|Default|SetnewLevelNumber NewParam))
  (SaveGame|SaveGametoSlot self "LevelNumberSlot")
  (return _output_get))

(fn LoadLevelNumber
  (bind _returnvalue (SaveGame|DoesSaveGameExist "LevelNumberSlot"))
  (if _returnvalue
    (bind _returnvalue_2 (SaveGame|LoadGamefromSlot "LevelNumberSlot"))
    (bind _asbp_save_level_number_and_name (Utilities|Casting|CastToBP_SaveLevelNumberAndName _returnvalue_2))
    (bind _output_get (Variables|Default|SetnewLevelNumber (Variables|BP_SaveLevelNumberAndName_C|GetnewLevelNumber _asbp_save_level_number_and_name)))
    (return _output_get)))

(fn SaveLevelName
  (params (NewParam :type Name))
  (bind _output_get (Variables|Default|SetnewLevelName NewParam))
  (SaveGame|SaveGametoSlot self "LevelNameSlot")
  (return _output_get))

(fn LoadLevelName
  (bind _returnvalue (SaveGame|DoesSaveGameExist "LevelNameSlot"))
  (if _returnvalue
    (bind _returnvalue_2 (SaveGame|LoadGamefromSlot "LevelNameSlot"))
    (bind _asbp_save_level_number_and_name (Utilities|Casting|CastToBP_SaveLevelNumberAndName _returnvalue_2))
    (bind _output_get (Variables|Default|SetnewLevelName (Variables|BP_SaveLevelNumberAndName_C|GetnewLevelName _asbp_save_level_number_and_name)))
    (return _output_get)))